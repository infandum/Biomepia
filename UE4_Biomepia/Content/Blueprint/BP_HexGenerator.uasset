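; Hex map generator that rebuilds a hexagon-shaped field of HexagonTile child actors in the construction script.
; GenerateHexagonalMap clears old tiles, then walks outward ring by ring from the center, filling each side between corners and storing each tile's index, transform and normalized UV.
; GenerateHeightFromMap samples the height texture at each UV, shapes the greyscale with a multiplier and exponent, then sets tile elevation and an elevation-tinted dynamic material.
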(event EventBeginPlay)

(event Collision|EventActorBeginOverlap
  (params (OtherActor :type Actor%20Object%20Reference)))

(event EventTick
  (params (DeltaSeconds :type Float%20%28single-precision%29)))

(fn ConstructionScript
  (CallFunction|GenerateHexagonalMap)
  (CallFunction|GenerateHeightfromMap)
  (Development|PrintString (Utilities|String|ToString(Integer) (Utilities|Array|Length (Actor|GetAllChildActors true)))))

(fn PointAroundCircle
  (params (Rad :type Float%20%28single-precision%29) (Radius :type Float%20%28single-precision%29))
  (return (Math|Vector|MakeVector (* (Math|Trig|Sin(Radians) Rad) Radius) (* (Math|Trig|Cos(Radians) Rad) Radius) 0.0)))

(fn HexagonCorners
  (params (center :type Vector) (Size :type Float%20%28single-precision%29) (Side :type Integer) (IsPointy :type Boolean))
  (bind _position (CallFunction|PointAroundCircle (Math|Trig|DegreesToRadians (+ (* 6e+01 (Math|Conversions|ToFloat(Integer) Side)) 3e+01)) Size))
  (return (+ center _position)))

(fn GenerateTile
  (params (Index :type Int%20Vector%20Structure) (Transform :type Transform))
  (bind _tilesize (Variables|Tile|GetTileSize))
  (bind _radius (Variables|Generator|GetRadius))
  (bind _returnvalue (Math|Conversions|ToFloat(Integer) _radius))
  (bind _returnvalue_2 (* _returnvalue _tilesize))
  (LocalVariables|Set2DIndex Index)
  (bind _output_get (LocalVariables|SetTrans Transform))
  (LocalVariables|SetUVIndex (Math|Vector2D|MakeVector2D (Math|Float|Clamp(Float) (/ (+ (/ (.x (.Location (Math|Transform|BreakTransform _output_get))) _returnvalue_2) 1.0) 2.0) 0.0 0.99999) (Math|Float|Clamp(Float) (/ (+ (/ (.y (.Location (Math|Transform|BreakTransform _output_get))) _returnvalue_2) 1.0) 2.0) 0.0 0.99999)))
  (bind _returnvalue_3 (AddComponent|AddChildActorComponent false (LocalVariables|GetTrans)))
  (ChildActorComponent|SetChildActorClass _returnvalue_3 (Variables|Tile|GetTileActor))
  (bind _ashexagon_tile (Utilities|Casting|CastToHexagonTile (Variables|/Script/Engine.ChildActorComponent|GetChildActor _returnvalue_3)))
  (Class|HexagonTile|SetTileData _ashexagon_tile (Math|Conversions|ToVector(Float) (LocalVariables|Get2DIndex)) (LocalVariables|GetUVIndex))
  (Utilities|Array|Add (Variables|Generator|GetHexTiles) _ashexagon_tile)
  (Utilities|Array|Add (Variables|Generator|GetTilesData) (Utilities|Struct|MakeHexTileStructure (Utilities|String|StringToName (Utilities|String|Append (LocalVariables|GetHexName) (Utilities|String|ToString(Integer) (LocalVariables|Get2DIndex)))) (LocalVariables|GetTrans) (LocalVariables|Get2DIndex) (LocalVariables|GetUVIndex) 0.0)))

(fn GenerateHexagonalMap
  (for _array_element (Actor|GetAllChildActors true)
    (Transformation|DetachFromActor _array_element "KeepRelative" "KeepRelative" "KeepRelative")
    (Components|DestroyComponent (Variables|/Script/Engine.Actor|GetRootComponent _array_element))
    (Components|DestroyComponent (Variables|/Script/Engine.Actor|GetRootComponent _array_element))
    (Actor|DestroyActor _array_element))
  (Utilities|Array|Clear (Variables|Generator|GetHexTiles))
  (Utilities|Array|Clear (Variables|Generator|GetTilesData))
  (CallFunction|GenerateTile)
  (for _index (range 1 (Variables|Generator|GetRadius))
    (LocalVariables|SetRadiusIndex _index)
    (for _index_2 (range 1 6)
      (bind _output_get (LocalVariables|SetDirectionIndex _index_2))
      (bind _position (CallFunction|PointAroundCircle (Math|Trig|DegreesToRadians (+ (* _output_get 6e+01) 3e+01)) (* (LocalVariables|GetRadiusIndex) (Variables|Tile|GetTileSize))))
      (bind _output_get_2 (LocalVariables|SetlocalPos _position))
      (Utilities|FlowControl|Sequence
        (:then_0
          (if (> (.X (Math|Vector|BreakVector _output_get_2)) 0.0)
            (LocalVariables|SetIndex (Utilities|Struct|MakeIntVector (LocalVariables|GetRadiusIndex) 0 0))
            (else
              (LocalVariables|SetIndex (Utilities|Struct|MakeIntVector (* (LocalVariables|GetRadiusIndex) -1) 0 0))))
          (if (and (!= (LocalVariables|GetDirectionIndex) 1) (!= (LocalVariables|GetDirectionIndex) 4))
            (if (> (.Y (Math|Vector|BreakVector (LocalVariables|GetlocalPos))) 0.0)
              (LocalVariables|SetIndex (Utilities|Struct|MakeIntVector (.x (LocalVariables|GetIndex)) (LocalVariables|GetRadiusIndex) 0))
              (else
                (LocalVariables|SetIndex (Utilities|Struct|MakeIntVector (.x (LocalVariables|GetIndex)) (* (LocalVariables|GetRadiusIndex) -1) 0)))))
          (CallFunction|GenerateTile (LocalVariables|GetIndex) (Math|Transform|MakeTransform (LocalVariables|GetlocalPos)))
          (for _index_3 (range 1 (- (LocalVariables|GetRadiusIndex) 1))
            (bind _output_get_3 (LocalVariables|SetArmIndex _index_3))
            (bind _pos (CallFunction|HexagonCorners (LocalVariables|GetlocalPos) (* (Math|Conversions|ToFloat(Integer) _output_get_3) (Variables|Tile|GetTileSize)) (Math|Integer|%(Integer) (+ (LocalVariables|GetDirectionIndex) 2) 6) false))
            (if (> (.y (LocalVariables|GetlocalPos)) 0.0)
              (LocalVariables|SetIndex (Utilities|Struct|MakeIntVector (.x (LocalVariables|GetIndex)) (LocalVariables|GetArmIndex) 0))
              (else
                (LocalVariables|SetIndex (Utilities|Struct|MakeIntVector (.x (LocalVariables|GetIndex)) (* (LocalVariables|GetArmIndex) -1) 0))))
            (CallFunction|GenerateTile (LocalVariables|GetIndex) (Math|Transform|MakeTransform _pos)))))))
  (return))

(fn GenerateHeightfromMap
  (for (_array_element _array_index) (Variables|Generator|GetHexTiles)
    (LocalVariables|SetTileData (Utilities|Array|Get(acopy) (Variables|Generator|GetTilesData) _array_index))
    (bind _output_get (LocalVariables|SetHexTile _array_element))
    (bind _returnvalue (Class|Texture2DHelper|GetColorfromTexture2D (Variables|HeightMap|GetHeightMap) (Variables|/Script/UE4_Biomepia.HexagonTile|GetHeightUV _output_get)))
    (bind _output_get_2 (LocalVariables|SetElevation (Math|Float|Power (* (Class|Texture2DHelper|ColortoGreyScale _returnvalue) (Variables|HeightMap|GetHeightMultiplier)) (Variables|HeightMap|GetHeightGrowth))))
    (bind _output_get_3 (LocalVariables|SetHeight (* _output_get_2 (Variables|Tile|GetTileSize))))
    (Class|HexagonTile|SetElevation (LocalVariables|GetHexTile) _output_get_3)
    (bind _output_get_4 (LocalVariables|SetTileData (Utilities|Struct|MakeHexTileStructure (.name (LocalVariables|GetTileData)) (.transform (LocalVariables|GetTileData)) (.2d_index (LocalVariables|GetTileData)) (.uv_index (LocalVariables|GetTileData)) (LocalVariables|GetElevation))))
    (Utilities|Array|SetArrayElem (Variables|Generator|GetTilesData) _array_index _output_get_4)
    (bind _returnvalue_2 (Rendering|Material|CreateDynamicMaterialInstance (Variables|Default|GetBaseMaterial) "None" :!class /Script/Engine.KismetMaterialLibrary))
    (Rendering|Material|SetVectorParameterValue _returnvalue_2 "Color" (Math|Conversions|ToLinearColor(Float) (LocalVariables|GetElevation)) :!class /Script/Engine.MaterialInstanceDynamic)
    (Rendering|Material|SetMaterial (Variables|/Script/UE4_Biomepia.HexagonTile|GetMeshComponent (LocalVariables|GetHexTile)) 0 _returnvalue_2)))