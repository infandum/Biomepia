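; Hexagon map actor that visualizes key points of a hexagon shape, apparently as a test of the hexagon geometry helpers.
; The construction script builds the shape and adds scaled-down hexagon static meshes as markers at its corners and non-centroid rhombus centers.
; Triangle, trapezoid and average-centroid helpers sit unused in the graph, and there is no runtime logic.
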(event EventBeginPlay)

(event Collision|EventActorBeginOverlap
  (params (OtherActor :type Actor%20Object%20Reference)))

(event EventTick
  (params (DeltaSeconds :type Float%20%28single-precision%29)))

(fn ConstructionScript
  (bind _output_get (Variables|Default|SetHexagon (Utilities|Struct|MakeHexagonShape "0.000000,0.000000,0.000000" 57.5 57.5 true)))
  (for _array_element (Class|HexagonShapeFunctions|GetCorners _output_get)
    (bind _returnvalue (AddComponent|AddStaticMeshComponent false (Math|Transform|MakeTransform _array_element "0, 0, 0" "0.100000,0.100000,0.100000")))
    (Components|StaticMesh|SetStaticMesh _returnvalue "/Game/Geometry/Meshes/1M_Hexagon.1M_Hexagon"))
  (for _array_element_2 0
    (bind _returnvalue_2 (AddComponent|AddStaticMeshComponent false (Math|Transform|MakeTransform _array_element_2 "0, 0, 0" "0.100000,0.100000,0.100000")))
    (Components|StaticMesh|SetStaticMesh _returnvalue_2 "/Game/Geometry/Meshes/1M_Hexagon.1M_Hexagon"))
  (for _array_element_3 (Class|HexagonShapeFunctions|GetRhombusCenters _output_get false)
    (bind _returnvalue_3 (AddComponent|AddStaticMeshComponent false (Math|Transform|MakeTransform _array_element_3 "0, 0, 0" "0.100000,0.100000,0.100000")))
    (Components|StaticMesh|SetStaticMesh _returnvalue_3 "/Game/Geometry/Meshes/1M_Hexagon.1M_Hexagon"))
  (for _array_element_4 0
    (bind _returnvalue_4 (AddComponent|AddStaticMeshComponent false (Math|Transform|MakeTransform _array_element_4 "0, 0, 0" "0.100000,0.100000,0.100000")))
    (Components|StaticMesh|SetStaticMesh _returnvalue_4 "/Game/Geometry/Meshes/1M_Hexagon.1M_Hexagon")))