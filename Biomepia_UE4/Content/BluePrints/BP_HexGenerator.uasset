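; BP_HexGenerator is an actor that lays out a hexagonal pattern of tile meshes in its construction script.
; For each ring up to Radius, it adds static mesh components at six points from the PointAroundCircle trig helper and records them in Hexagons.
; Outer rings also add one raised tile via HexagonCorners on the first side, with a debug print.
; The edge-fill loop and IsPointy branch are disconnected, so the grid appears unfinished.
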(event EventBeginPlay)

(event Collision|EventActorBeginOverlap
  (params (OtherActor :type Actor%20Object%20Reference)))

(event EventTick
  (params (DeltaSeconds :type Float%20%28single-precision%29)))

(fn ConstructionScript
  (Utilities|Array|Clear (Variables|Default|GetHexagon_Tiles))
  (for _index (range 1 (Variables|Default|GetRadius))
    (for _index_2 (range 1 6)
      (bind _position (CallFunction|PointAroundCircle (Math|Trig|DegreesToRadians (+ (* _index_2 6e+01) 3e+01)) (* _index 1e+02)))
      (bind _output_get (LocalVariables|SetlocalPos _position))
      (Utilities|FlowControl|Sequence
        (:then_0
          (bind _returnvalue (AddComponent|AddStaticMeshComponent false (Math|Transform|MakeTransform _output_get)))
          (Components|StaticMesh|SetStaticMesh _returnvalue (Variables|Default|GetHexagon_Tile))
          (Utilities|Array|Add (Variables|Default|GetHexagons) (Utilities|Struct|MakeHexTileStructure "None" _returnvalue "0.000000,0.000000,0.000000|0.000000,0.000000,0.000000|1.000000,1.000000,1.000000" "(X=0.000000,Y=0.000000)" "(X=0.000000,Y=0.000000)"))
          (if (> _index 1)
            (if (== _index_2 1)
              (bind _pos (CallFunction|HexagonCorners (LocalVariables|GetlocalPos) (* (Math|Conversions|ToFloat(Integer) (stale _index)) 1e+02) (Math|Integer|%(Integer) (+ (stale _index) 1) 6) false))
              (bind _returnvalue_2 (AddComponent|AddStaticMeshComponent false))
              (Development|PrintString (Utilities|String|ToString(Vector) _pos))
              (Transformation|SetWorldLocation _returnvalue_2 (+ _pos "0, 0,100.000000") false true)
              (Components|StaticMesh|SetStaticMesh _returnvalue_2 (Variables|Default|GetHexagon_Tile))
              (Utilities|Array|Add (Variables|Default|GetHexagons) (Utilities|Struct|MakeHexTileStructure "None" _returnvalue_2 "0.000000,0.000000,0.000000|0.000000,0.000000,0.000000|1.000000,1.000000,1.000000" "(X=0.000000,Y=0.000000)" "(X=0.000000,Y=0.000000)")))))))))

(fn PointAroundCircle
  (params (Rad :type Float%20%28single-precision%29) (Radius :type Float%20%28single-precision%29))
  (return (Math|Vector|MakeVector (* (Math|Trig|Sin(Radians) Rad) Radius) (* (Math|Trig|Cos(Radians) Rad) Radius) 0.0)))

(fn HexagonCorners
  (params (center :type Vector) (Size :type Float%20%28single-precision%29) (Side :type Integer) (IsPointy :type Boolean))
  (bind _position (CallFunction|PointAroundCircle (Math|Trig|DegreesToRadians (+ (* 6e+01 (Math|Conversions|ToFloat(Integer) Side)) 3e+01)) Size))
  (return (+ _position center)))